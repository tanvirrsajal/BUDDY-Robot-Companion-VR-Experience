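; Player pawn that moves around the lab levels and lets the player talk to the BP_BuddyRobot AI companion.
; Tick applies movement, yaw and clamped camera pitch, and confines position to a box chosen by whether the level is Lobby.
; VoiceRecord press and release start and stop recording for transcription on BuddyAI.
; Interact line-traces from the camera for a BP_LabObject, interrupts Buddy's speech and asks it about that object.
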(event `self.ReceiveBeginPlay`
  (bind _returnvalue (`GameplayStatics.GetPlayerController` 0))
  (`WidgetBlueprintLibrary.SetInputMode_GameAndUIEx` _returnvalue null "DoNotLock" false)
  (set `PlayerController.bShowMouseCursor` true _returnvalue)
  (set `PlayerController.bEnableClickEvents` true _returnvalue))

(event `self.ReceiveTick`
  (params (DeltaSeconds :type "Float (single-precision)"))
  (`self.AddMovementInput` (`self.GetActorForwardVector`) (`self.GetInputAxisValue`))
  (`self.AddMovementInput` (`self.GetActorRightVector`) (`self.GetInputAxisValue`))
  (`self.K2_AddActorLocalRotation` (`KismetMathLibrary.MakeRotator` 0.0 0.0 (`self.GetInputAxisValue`)))
  (bind _returnvalue (`KismetStringLibrary.EqualEqual_StrStr` (stale _returnvalue_2) "Lobby"))
  (`self.K2_SetActorLocation` (`KismetMathLibrary.MakeVector` (`KismetMathLibrary.FClamp` (.x (`self.K2_GetActorLocation`)) (`KismetMathLibrary.SelectFloat` -280.0 -970.0 _returnvalue) (`KismetMathLibrary.SelectFloat` 250.0 970.0 _returnvalue)) (`KismetMathLibrary.FClamp` (.y (`self.K2_GetActorLocation`)) (`KismetMathLibrary.SelectFloat` -460.0 -970.0 _returnvalue) (`KismetMathLibrary.SelectFloat` -35.0 970.0 _returnvalue)) (`KismetMathLibrary.FClamp` (.z (`self.K2_GetActorLocation`)) (`KismetMathLibrary.SelectFloat` 10.0 10.0 _returnvalue) (`KismetMathLibrary.SelectFloat` 320.0 520.0 _returnvalue))) true)
  (`SceneComponent.K2_SetRelativeRotation` (`self.Camera`) (`KismetMathLibrary.MakeRotator` 0.0 (`KismetMathLibrary.FClamp` (+ (.pitch (`SceneComponent.RelativeRotation` (`self.Camera`))) (* (`self.GetInputAxisValue`) -1.0)) -80.0 80.0)) false false)
  (bind _returnvalue_2 (`GameplayStatics.GetCurrentLevelName` true)))

(event `InputAction|VoiceRecord`
  (params (Key :type "Key Structure"))
  (:`Pressed`
    (bind _outactors (`GameplayStatics.GetAllActorsOfClass` "/Game/BUDDY/Blueprints/BP_BuddyRobot.BP_BuddyRobot_C"))
    (bind _asbp_buddy_robot (cast `/Game/BUDDY/Blueprints/BP_BuddyRobot` (`|GetArrayItem` _outactors)))
    (`BuddyAIComponent.StartRecording` (`/Game/BUDDY/Blueprints/BP_BuddyRobot.BuddyAI` _asbp_buddy_robot))))

(event `InputAction|VoiceRecord`
  (params (Key :type "Key Structure"))
  (:`Released`
    (bind _outactors (`GameplayStatics.GetAllActorsOfClass` "/Game/BUDDY/Blueprints/BP_BuddyRobot.BP_BuddyRobot_C"))
    (bind _asbp_buddy_robot (cast `/Game/BUDDY/Blueprints/BP_BuddyRobot` (`|GetArrayItem` _outactors)))
    (`BuddyAIComponent.StopRecordingAndTranscribe` (`/Game/BUDDY/Blueprints/BP_BuddyRobot.BuddyAI` _asbp_buddy_robot))))

(event `InputAction|Interact`
  (params (Key :type "Key Structure"))
  (bind _returnvalue (`GameplayStatics.GetPlayerCameraManager` 0))
  (bind _returnvalue_2 (`PlayerCameraManager.GetCameraLocation` _returnvalue))
  (:`Pressed`
    (`|ExecutionSequence`
      (:`then_0`
        (bind _outhit (`KismetSystemLibrary.LineTraceSingle` :`Start` _returnvalue_2 :`End` (+ _returnvalue_2 (* (`KismetMathLibrary.GetForwardVector` (`PlayerCameraManager.GetCameraRotation` _returnvalue)) 3000.0)) :`TraceChannel` "TraceTypeQuery1" :`DrawDebugType` "ForOneFrame"))
        (bind _asbp_lab_object (cast `/Game/BUDDY/Blueprints/BP_LabObject` (`.HitActor` (`GameplayStatics.BreakHitResult` _outhit))))
        (bind _returnvalue_3 (`GameplayStatics.GetActorOfClass` "/Game/BUDDY/Blueprints/BP_BuddyRobot.BP_BuddyRobot_C"))
        (bind _buddyai (`/Game/BUDDY/Blueprints/BP_BuddyRobot.BuddyAI` _returnvalue_3))
        (`BuddyAIComponent.StopSpeaking` _buddyai)
        (`BuddyAIComponent.AskAboutObject` _buddyai (`/Game/BUDDY/Blueprints/BP_LabObject.ObjectName` _asbp_lab_object) (`/Game/BUDDY/Blueprints/BP_LabObject.ObjectDescription` _asbp_lab_object))))))

(fn `UserConstructionScript`)