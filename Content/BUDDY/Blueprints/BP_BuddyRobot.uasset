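; BP_BuddyRobot is an AI assistant robot that greets the player on BeginPlay by asking its BuddyAI component for a short self-introduction.
; AI responses are written to the ChestPanel's WBP_BuddyScreen and set the talking state in ABP_Buddy, which clears once speaking finishes.
; Tick copies the AI's movement state into the AnimBP to drive walking.
; Distance-based panel visibility logic exists but is unwired, and overlap events are empty.
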(event `OnSpeakingDone_Event_0`
  (if (not (`BuddyAIComponent.bSpeaking` (`self.BuddyAI`)))
    (bind _asabp_buddy (cast `/Game/BUDDY/ABP_Buddy` (`SkeletalMeshComponent.GetAnimInstance` (`self.RobotBody`))))
    (set `/Game/BUDDY/ABP_Buddy.IsTalking` false _asabp_buddy)))

(event `self.ReceiveBeginPlay`
  (add `BuddyAIComponent.OnResponse` (`self.BuddyAI`) (delegate `OnResponse_Event_0`))
  (`|ExecutionSequence`
    (:`then_0`
      (bind _aswbp_buddy_screen (cast `/Game/BUDDY/Widgets/WBP_BuddyScreen` (`WidgetComponent.GetUserWidgetObject` (`self.ChestPanel`))))
      (set `/Game/BUDDY/Widgets/WBP_BuddyScreen.BuddyRef ` self _aswbp_buddy_screen)
      (`BuddyAIComponent.AskFollowUp` (`self.BuddyAI`) "\"Introduce yourself in one sentence. Greet them, say your name and that you are here to help. Keep it short\""))
    (:`then_1`
      _))
  (add `BuddyAIComponent.OnSpeakingDone` (`self.BuddyAI`) (delegate `OnSpeakingDone_Event_0`)))

(event `OnResponse_Event_0`
  (params (ResponseText :type String))
  (bind _aswbp_buddy_screen (cast `/Game/BUDDY/Widgets/WBP_BuddyScreen` (`WidgetComponent.GetUserWidgetObject` (`self.ChestPanel`))))
  (set `/Game/BUDDY/Widgets/WBP_BuddyScreen.ResponseString` (`KismetTextLibrary.Conv_TextToString` (`KismetTextLibrary.Conv_StringToText` ResponseText)) _aswbp_buddy_screen)
  (bind _asabp_buddy (cast `/Game/BUDDY/ABP_Buddy` (`SkeletalMeshComponent.GetAnimInstance` (`self.RobotBody`))))
  (set `/Game/BUDDY/ABP_Buddy.IsTalking` true _asabp_buddy))

(event `self.ReceiveActorBeginOverlap`
  (params (OtherActor :type "Actor Object Reference")))

(event `self.ReceiveActorEndOverlap`
  (params (OtherActor :type "Actor Object Reference")))

(event `self.ReceiveTick`
  (params (DeltaSeconds :type "Float (single-precision)"))
  (bind _asabp_buddy (cast `/Game/BUDDY/ABP_Buddy` (`SkeletalMeshComponent.GetAnimInstance` (`self.RobotBody`))))
  (set `/Game/BUDDY/ABP_Buddy.IsWalking` (`BuddyAIComponent.bIsMoving` (`self.BuddyAI`)) _asabp_buddy))

(fn `UserConstructionScript`)