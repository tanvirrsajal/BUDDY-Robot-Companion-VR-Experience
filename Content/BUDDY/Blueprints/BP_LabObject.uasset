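; BP_LabObject is a named lab object that highlights when the VR player comes near.
; On BeginPlay it binds the InteractZone begin overlap, which turns on HighlightLight and sets PlayerNearby for BP_VRPlayer.
; The end-overlap handler reverses both and prints the object name, but its only bind sits inside itself, so nothing shown hooks it up.
; A BP_BuddyRobot lookup and an AskAboutObject call passing name and description are present but never run.
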(event `self.ReceiveBeginPlay`
  (add `PrimitiveComponent.OnComponentBeginOverlap` (`self.InteractZone`) (delegate `OnComponentBeginOverlap_Event_0`)))

(event `OnComponentBeginOverlap_Event_0`
  (params (OverlappedComponent :type "PrimitiveComponent Object Reference") (OtherActor :type "Actor Object Reference") (OtherComp :type "PrimitiveComponent Object Reference") (OtherBodyIndex :type Integer) (bFromSweep :type Boolean) (SweepResult :type "HitResult Structure (by ref)"))
  (cast `/Game/BUDDY/Blueprints/BP_VRPlayer` OtherActor)
  (`LightComponent.SetIntensity` (`self.HighlightLight`) 800.0)
  (set `self.bPlayerNearby` true))

(event `OnActorEndOverlap_Event_0` :!signature `self.OnActorEndOverlap`
  (params (OverlappedActor :type "Actor Object Reference") (OtherActor :type "Actor Object Reference"))
  (add `self.OnActorEndOverlap` (delegate `OnActorEndOverlap_Event_0`))
  (cast `/Game/BUDDY/Blueprints/BP_VRPlayer` OtherActor)
  (`LightComponent.SetIntensity` (`self.HighlightLight`) 0.0)
  (set `self.bPlayerNearby` false)
  (`KismetSystemLibrary.PrintString` (`KismetStringLibrary.Concat_StrStr` "Left: " (`self.ObjectName`)) true true (struct :`G` 0.66 :`B` 1.0 :`A` 1.0) 5.0))

(fn `UserConstructionScript`)